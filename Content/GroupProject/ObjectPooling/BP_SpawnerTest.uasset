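; BP_SpawnerTest is a test actor that periodically spawns objects through the project's object pooling system.
; On BeginPlay it finds the BP_ObjectPoolinSystem actor in the level and stores it as the pool.
; Tick accumulates a timer, and every five seconds calls SpawnFromPool with a random object code of 0 or 1 at a random XY point near the world origin.
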(event EventBeginPlay
  (bind _returnvalue (Actor|GetActorOfClass "/Game/GroupProject/ObjectPooling/BP_ObjectPoolinSystem.BP_ObjectPoolinSystem_C"))
  (Variables|Default|SetPool _returnvalue))

(event Collision|EventActorBeginOverlap
  (params (OtherActor :type Actor%20Object%20Reference)))

(event EventTick
  (params (DeltaSeconds :type Float%20%28single-precision%29))
  (bind _output_get (Variables|Default|Settimer (+ (Variables|Default|Gettimer) DeltaSeconds)))
  (if (>= _output_get 5.0)
    (Variables|Default|Settimer 0.0)
    (Class|ObjectPoolingSystem|SpawnfromPool (Variables|Default|GetPool) (Math|Random|RandomIntegerinRange 0 1) (Math|Transform|MakeTransform (Math|Vector|MakeVector (Math|Random|RandomFloatinRange -1e+02 1e+02) (Math|Random|RandomFloatinRange -1e+02 1e+02) 0.0)))))

(fn ConstructionScript)