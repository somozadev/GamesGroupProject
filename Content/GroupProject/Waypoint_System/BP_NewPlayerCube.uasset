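; BP_NewPlayerCube is a player character that can jump and request a waypoint route to a random destination.
; T or the gamepad top face button picks a random BP_Destination actor and passes its location to the BPCWaypoint component's waypoint creation, with distance, update and height-offset settings.
; A PlayerHealth component supplies the health value, which is printed on BeginPlay and whenever damage is received.
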(event EventBeginPlay
  (Development|PrintString (Utilities|String|ToString(Float) (Variables|/Script/GamesGroupProject.PlayerHealthComponent|GetHealth (Variables|Default|GetPlayerHealth)))))

(event Collision|EventActorBeginOverlap
  (params (OtherActor :type Actor%20Object%20Reference)))

(event EventTick
  (params (DeltaSeconds :type Float%20%28single-precision%29)))

(event Game|Damage|EventAnyDamage
  (params (Damage :type Float%20%28single-precision%29) (DamageType :type Damage%20Type%20Object%20Reference) (InstigatedBy :type Controller%20Object%20Reference) (DamageCauser :type Actor%20Object%20Reference))
  (Development|PrintString (Utilities|String|ToString(Float) (Variables|/Script/GamesGroupProject.PlayerHealthComponent|GetHealth (Variables|Default|GetPlayerHealth)))))

(event Input|KeyboardEvents|T
  (params (Key :type Key%20Structure :default "None"))
  (:Pressed
    (bind _outactors (Actor|GetAllActorsOfClass "/Game/GroupProject/Waypoint_System/BP_Destination.BP_Destination_C"))
    (Default|CreateWayoint (Variables|Default|GetBPC_Waypoint) (Transformation|GetActorLocation (.OutItem (Utilities|Array|Random _outactors))) 3e+02 0.2 2.5e+02 5e+01)))

(event Input|GamepadEvents|GamepadFaceButtonTop
  (params (Key :type Key%20Structure :default "None"))
  (:Pressed
    (bind _outactors (Actor|GetAllActorsOfClass "/Game/GroupProject/Waypoint_System/BP_Destination.BP_Destination_C"))
    (Default|CreateWayoint (Variables|Default|GetBPC_Waypoint) (Transformation|GetActorLocation (.OutItem (Utilities|Array|Random _outactors))) 3e+02 0.2 2.5e+02 5e+01)))

(event Input|KeyboardEvents|SpaceBar
  (params (Key :type Key%20Structure :default "None"))
  (:Pressed
    (Character|Jump)))

(event Input|GamepadEvents|GamepadFaceButtonBottom
  (params (Key :type Key%20Structure :default "None"))
  (:Pressed
    (Character|Jump)))

(fn ConstructionScript)