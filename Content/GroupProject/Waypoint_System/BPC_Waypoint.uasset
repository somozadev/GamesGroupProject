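; Waypoint component that shows its owning actor a navigation path to a goal location as a trail of thin cylinders.
; GetPath finds a navmesh path, requested via a server event on clients, then builds a spline and spline meshes on a spawned BP_WaypointManager.
; A looping timer rebuilds the trail when the owner strays from its start.
; The trail clears near the goal or when a three-second retriggerable delay expires.
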(event Custom|CreateWayoint
  (params (GoalLocation :type Vector) (GoalDistance :type Float%20%28double-precision%29) (UpdateIntrerval :type Float%20%28double-precision%29) (UpdateDistance :type Float%20%28double-precision%29) (Z_Offset :type Float%20%28double-precision%29))
  (Variables|Default|SetGoalLocation GoalLocation)
  (Variables|Default|SetGoalDistance GoalDistance)
  (Variables|Default|SetUpdateIntrerval UpdateIntrerval)
  (Variables|Default|SetUpdateDistance UpdateDistance)
  (Variables|Default|SetZ_Offset Z_Offset)
  (Utilities|IsValid (Variables|Default|GetBP_WaypointManager)
    (:Is%20Valid
      (Utilities|IsValid (Variables|Default|GetSplineComponent)
        (:Is%20Valid
          (Spline|ClearSplinePoints (Variables|Default|GetSplineComponent) true))
        (:Is%20Not%20Valid
          (bind _returnvalue (Game|AddComponentbyClass (Variables|Default|GetBP_WaypointManager) "/Script/Engine.SplineComponent" false))
          (Variables|Default|SetSplineComponent _returnvalue)))
      (Utilities|Array|Clear (Variables|Default|GetPath))
      (if (Networking|IsServer)
        (CallFunction|GetPath (Variables|Default|GetGoalLocation))
        (else
          (CallFunction|SrverGetPath (Variables|Default|GetGoalLocation)))))
    (:Is%20Not%20Valid
      (bind _returnvalue_2 (Game|SpawnActorfromClass "/Game/GroupProject/Waypoint_System/BP_WaypointManager.BP_WaypointManager_C" (Math|Transform|MakeTransform "0, 0, 0") "AlwaysSpawn" "MultiplyWithRoot" 0 0))
      (Variables|Default|SetBP_WaypointManager _returnvalue_2))))

(event Custom|GetPath
  (params (TargetLocation :type Vector))
  (bind _returnvalue (Class|NavigationSystemV1|FindPathtoLocationSynchronously (Transformation|GetActorLocation (Components|GetOwner)) TargetLocation 0 0))
  (if (and (Utilities|IsValid _returnvalue) (> (Utilities|Array|Length (Variables|/Script/NavigationSystem.NavigationPath|GetPathPoints _returnvalue)) 0))
    (CallFunction|OwnerrCreateWaypoint (Variables|/Script/NavigationSystem.NavigationPath|GetPathPoints _returnvalue))
    (else
      (CallFunction|OwnerResetDelay))))

(event Custom|SrverGetPath
  (params (TargetLocation :type Vector))
  (CallFunction|GetPath TargetLocation))

(event Custom|OwnerrCreateWaypoint
  (params (Path :type Array%20of%20Vectors))
  (bind _returnvalue (Math|Vector2D|MakeVector2D 0.03 0.03))
  (bind _splinecomponent (Variables|Default|GetSplineComponent))
  (bind _splinecomponent_2 (Variables|Default|GetSplineComponent))
  (bind _bp_waypointmanager (Variables|Default|GetBP_WaypointManager))
  (bind _splinecomponent_3 (Variables|Default|GetSplineComponent))
  (bind _splinecomponent_4 (Variables|Default|GetSplineComponent))
  (bind _output_get (Variables|Default|SetPath Path))
  (Variables|Default|SetWaypointStartLocation (Utilities|Array|Get(acopy) _output_get))
  (Default|RemoveWaypoint (Variables|Default|GetBP_WaypointManager))
  (for (_array_element _array_index) (Variables|Default|GetPath)
    (Spline|AddSplinePointatIndex _splinecomponent_4 (+ _array_element (Math|Vector|MakeVector 0.0 0.0 (Variables|Default|GetZ_Offset))) _array_index "World" false)
    (Spline|SetSplinePointType _splinecomponent_4 _array_index "Constant" false))
  (Spline|UpdateSpline (Variables|Default|GetSplineComponent))
  (for _index (range 0 (- (Utilities|Array|LastIndex (Variables|Default|GetPath)) 1))
    (bind _returnvalue_2 (Game|AddComponentbyClass (Variables|Default|GetBP_WaypointManager) "/Script/Engine.SplineMeshComponent" false))
    (Utilities|Array|Add (Variables|/Game/GroupProject/Waypoint_System/BP_WaypointManager.BP_WaypointManager_C|GetSplineMeshes (Variables|Default|GetBP_WaypointManager)) _returnvalue_2)
    (Transformation|SetMobility _returnvalue_2 "Movable")
    (Components|StaticMesh|SetStaticMesh _returnvalue_2 "/Game/GroupProject/Waypoint_System/Meshes/Shape_Cylinder.Shape_Cylinder")
    (SplineMesh|SetStartandEnd _returnvalue_2 (Spline|GetLocationatSplinePoint _splinecomponent_2 _index "World") (Spline|GetTangentatSplinePoint _splinecomponent_2 _index "World") (Spline|GetLocationatSplinePoint _splinecomponent (+ _index 1) "World") (Spline|GetTangentatSplinePoint _splinecomponent (+ _index 1) "World") false :!class /Script/Engine.SplineMeshComponent)
    (SplineMesh|SetStartScale _returnvalue_2 _returnvalue true :!class /Script/Engine.SplineMeshComponent)
    (SplineMesh|SetEndScale _returnvalue_2 _returnvalue true :!class /Script/Engine.SplineMeshComponent))
  (if (Utilities|Time|IsValidTimerHandle (Variables|Default|GetWaypointTimerHandle))
    _
    (else
      (bind _returnvalue_3 (Utilities|Time|SetTimerbyFunctionName 0 "WaypointTimer" (Variables|Default|GetUpdateIntrerval) true))
      (Variables|Default|SetWaypointTimerHandle _returnvalue_3)))
  (Utilities|FlowControl|RetriggerableDelay 3.0)
  (Utilities|IsValid _bp_waypointmanager
    (:Is%20Valid
      (Default|RemoveWaypoint _bp_waypointmanager))
    (:Is%20Not%20Valid
      _))
  (Utilities|IsValid _splinecomponent_3
    (:Is%20Valid
      (Spline|ClearSplinePoints _splinecomponent_3 true))
    (:Is%20Not%20Valid
      _))
  (if (Utilities|Time|IsValidTimerHandle (Variables|Default|GetWaypointTimerHandle))
    (Utilities|Time|ClearandInvalidateTimerbyHandle (Variables|Default|GetWaypointTimerHandle))))

(event Custom|WaypointTimer
  (bind _bp_waypointmanager (Variables|Default|GetBP_WaypointManager))
  (bind _splinecomponent (Variables|Default|GetSplineComponent))
  (bind _waypointtimerhandle (Variables|Default|GetWaypointTimerHandle))
  (bind (_updatewaypoint _removewaypoint) (CallFunction|CheckUpdateDistance))
  (if _updatewaypoint
    (CallFunction|CreateWayoint (Variables|Default|GetGoalLocation) (Variables|Default|GetGoalDistance) (Variables|Default|GetUpdateIntrerval) (Variables|Default|GetUpdateDistance) (Variables|Default|GetZ_Offset))
    (elif _removewaypoint
      (Utilities|IsValid _bp_waypointmanager
        (:Is%20Valid
          (Default|RemoveWaypoint _bp_waypointmanager))
        (:Is%20Not%20Valid
          _))
      (Utilities|IsValid _splinecomponent
        (:Is%20Valid
          (Spline|ClearSplinePoints _splinecomponent true))
        (:Is%20Not%20Valid
          _))
      (if (Utilities|Time|IsValidTimerHandle _waypointtimerhandle)
        (Utilities|Time|ClearandInvalidateTimerbyHandle _waypointtimerhandle)))))

(event Custom|OwnerResetDelay
  (bind _bp_waypointmanager (Variables|Default|GetBP_WaypointManager))
  (bind _splinecomponent (Variables|Default|GetSplineComponent))
  (bind _waypointtimerhandle (Variables|Default|GetWaypointTimerHandle))
  (Utilities|FlowControl|RetriggerableDelay 3.0)
  (Utilities|IsValid _bp_waypointmanager
    (:Is%20Valid
      (Default|RemoveWaypoint _bp_waypointmanager))
    (:Is%20Not%20Valid
      _))
  (Utilities|IsValid _splinecomponent
    (:Is%20Valid
      (Spline|ClearSplinePoints _splinecomponent true))
    (:Is%20Not%20Valid
      _))
  (if (Utilities|Time|IsValidTimerHandle _waypointtimerhandle)
    (Utilities|Time|ClearandInvalidateTimerbyHandle _waypointtimerhandle)))

(fn CheckUpdateDistance
  (bind _goaldistance (Variables|Default|GetGoalDistance))
  (bind _updatedistance (Variables|Default|GetUpdateDistance))
  (LocalVariables|SetLocalPlayerLocation (Transformation|GetActorLocation (Components|GetOwner)))
  (if (< (Class|KismetMathLibrary|VectorDistanceSquared (Variables|Default|GetGoalLocation) (LocalVariables|GetLocalPlayerLocation)) (* _goaldistance _goaldistance))
    (return false true)
    (elif (> (Class|KismetMathLibrary|VectorDistanceSquared (Variables|Default|GetWaypointStartLocation) (LocalVariables|GetLocalPlayerLocation)) (* _updatedistance _updatedistance))
      (return true false)
      (else
        (return false false)))))