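; Component that tracks which card in the inventory is active, cycled with the CardSelectLeft and CardSelectRight inputs.
; BeginPlay caches the world inventory, player cube and UI_Test widget.
; Each press moves the index with wraparound, unpacks that InventoryActive entry's X as card ID and Y as cards left, and prints the count.
; SetActiveCard only returns the ID; Fire and ChangeCurrentCardIndex are unfinished stubs.
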(event EventBeginPlay
  (Variables|Default|SetCardDataTable "/Game/GroupProject/Inventory/CardHolds.CardHolds")
  (bind _returnvalue (Actor|GetActorOfClass "/Script/GamesGroupProject.InventoryInWorldComp"))
  (Variables|Default|SetInventory _returnvalue)
  (bind _returnvalue_2 (Actor|GetActorOfClass "/Game/GroupProject/Player/BP_NewPlayerCube.BP_NewPlayerCube_C"))
  (Variables|Default|SetPlayer _returnvalue_2)
  (bind _foundwidgets (Widget|GetAllWidgetsOfClass "/Game/GroupProject/UI/UI_Test.UI_Test_C" false))
  (Variables|Default|SetWidget (Utilities|Array|Get(acopy) _foundwidgets)))

(event Input|ActionEvents|InputActionCardSelectLeft
  (params (Key :type Key%20Structure :default "None"))
  (:Pressed
    (CallFunction|Leftcard)
    (CallFunction|SetActiveCard)))

(event Input|ActionEvents|InputActionCardSelectRight
  (params (Key :type Key%20Structure :default "None"))
  (:Pressed
    (CallFunction|RightCard)
    (CallFunction|SetActiveCard)))

(event Input|KeyboardEvents|DebugKeyX
  (params (Key :type Key%20Structure :default "None") (ActionValue :type Input%20Action%20Value%20Structure)))

(fn GetCardData
  (params (CardID :type Integer))
  (bind _currentcardindex (Variables|Default|GetCurrentcardIndex))
  (bind _inventory (Variables|Default|GetInventory))
  (bind _inventoryactive (Variables|/Script/GamesGroupProject.InventoryInWorldComp|GetInventoryActive _inventory))
  (bind _output (Utilities|Array|Get(acopy) _inventoryactive _currentcardindex))
  (bind (_x _y) (Math|Vector2D|BreakVector2D _output))
  (if true
    (Variables|Default|SetXvalue (Math|Float|Truncate _x))
    (Variables|Default|SetYvalue (Math|Float|Truncate _y))))

(fn ChangeCurrentCardIndex
  (params (ActiveIndex :type Integer)))

(fn RightCard
  (if (== (Variables|Default|GetCurrentcardIndex) (- (Utilities|Array|Length (Variables|/Script/GamesGroupProject.InventoryInWorldComp|GetInventoryActive (Variables|Default|GetInventory))) 1))
    (bind _output_get (Variables|Default|SetCurrentcardIndex 0))
    (CallFunction|GetCardData _output_get)
    (Development|PrintString (Utilities|String|Append (Utilities|String|ToString(Integer) (Variables|Default|GetYvalue)) "cardsleft"))
    (else
      (bind _output_get_2 (Variables|Default|SetCurrentcardIndex (+ (Variables|Default|GetCurrentcardIndex) 1)))
      (CallFunction|GetCardData _output_get_2)
      (Development|PrintString (Utilities|String|Append (Utilities|String|ToString(Integer) (Variables|Default|GetYvalue)) "cardsleft")))))

(fn Leftcard
  (if (== (Variables|Default|GetCurrentcardIndex) 0)
    (bind _output_get (Variables|Default|SetCurrentcardIndex (- (Utilities|Array|Length (Variables|/Script/GamesGroupProject.InventoryInWorldComp|GetInventoryActive (Variables|Default|GetInventory))) 1)))
    (CallFunction|GetCardData _output_get)
    (Development|PrintString (Utilities|String|Append (Utilities|String|ToString(Integer) (Variables|Default|GetYvalue)) "cards left"))
    (else
      (bind _output_get_2 (Variables|Default|SetCurrentcardIndex (- (Variables|Default|GetCurrentcardIndex) 1)))
      (CallFunction|GetCardData _output_get_2)
      (Development|PrintString (Utilities|String|Append (Utilities|String|ToString(Integer) (Variables|Default|GetYvalue)) "cards left")))))

(fn GetArraySize
  (Variables|Default|SetArraySize (Utilities|Array|Length (Variables|/Script/GamesGroupProject.InventoryInWorldComp|GetInventoryActive (Variables|Default|GetInventory)))))

(fn SetActiveCard
  (return (Variables|Default|GetXvalue)))

(fn Fire
  (if (== (Variables|Default|GetXvalue) 0)
    _))