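; BP_Door is a level exit door that swings open and loads Level2 when its OnDoorOpenedBP event fires.
; A Timeline's Door track drives a Lerp that yaws the static mesh to a right angle.
; The same Update chain, rather than Finished, runs a delay, plays a 2D sound and starts the WB_Fadein widget's transition.
; A second short delay then precedes opening the level by name.
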(event EventOnDoorOpenedBP
  ;[1 1 1] Door
  (bind _door (Timeline|Timeline Play)
    (:Update
      (Transformation|SetRelativeRotation (Variables|Default|GetStaticMesh) (Math|Rotator|MakeRotator 0.0 0.0 (Math|Float|Lerp 0.0 9e+01 _door)) false false)
      (Utilities|FlowControl|Delay 2.0)
      (Audio|PlaySound2D 0 1.0 1.0 0.0 0 0)
      (bind _returnvalue (UserInterface|CreateWidget "/Game/GroupProject/Level_01/Blueprints/WB_Fadein.WB_Fadein_C"))
      (UserInterface|Viewport|AddtoViewport _returnvalue 0)
      (Default|Fadetransition _returnvalue)
      (Utilities|FlowControl|Delay 0.5)
      (Game|OpenLevel(byName) "Level2"))))

(fn ConstructionScript)