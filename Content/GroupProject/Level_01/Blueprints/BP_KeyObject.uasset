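; BP_KeyObject is a key pickup that the player can interact with in the level.
; On BeginPlay it creates a WB_interactbutton prompt, shown and hidden as the player character enters or leaves its Box trigger.
; Interacting calls PickupKeyMessage on its referenced Door, then destroys the key actor.
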(event OnComponentBeginOverlap(Box)
  (params (OverlappedComponent :type Primitive%20Component%20Object%20Reference) (OtherActor :type Actor%20Object%20Reference) (OtherComp :type Primitive%20Component%20Object%20Reference) (OtherBodyIndex :type Integer) (bFromSweep :type Boolean) (SweepResult :type Hit%20Result%20Structure%20%28by%20ref%29))
  (if (== OtherActor (Game|GetPlayerCharacter 0))
    (UserInterface|Viewport|AddtoViewport (Variables|Default|GetPrompt) 0)))

(event OnComponentEndOverlap(Box)
  (params (OverlappedComponent :type Primitive%20Component%20Object%20Reference) (OtherActor :type Actor%20Object%20Reference) (OtherComp :type Primitive%20Component%20Object%20Reference) (OtherBodyIndex :type Integer))
  (if (== (Game|GetPlayerCharacter 0) OtherActor)
    (Widget|RemovefromParent (Variables|Default|GetPrompt))))

(event EventBeginPlay
  (bind _returnvalue (UserInterface|CreateWidget "/Game/GroupProject/Level_01/Blueprints/WB_interactbutton.WB_interactbutton_C"))
  (Variables|Default|SetPrompt _returnvalue))

(event Collision|EventActorBeginOverlap
  (params (OtherActor :type Actor%20Object%20Reference)))

(event EventTick
  (params (DeltaSeconds :type Float%20%28single-precision%29)))

(event EventInteract
  (Class|BPIDoor|PickupKey(Message) (Variables|Default|GetDoor))
  (Actor|DestroyActor))

(fn ConstructionScript)