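; BP_PlayerCubeRespawnTest is a test player Blueprint with a PlayerHealth component, though it holds no respawn logic despite its name.
; It prints current health at BeginPlay and on AnyDamage, without changing it in this graph.
; The Turn axis drives controller yaw.
; LookUp is left unwired, with its pitch node disconnected; a note says vertical look makes a floating-movement pawn fly.
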(event EventBeginPlay
  (Development|PrintString (Utilities|String|ToString(Float) (Variables|/Script/GamesGroupProject.PlayerHealthComponent|GetHealth (Variables|Default|GetPlayerHealth)))))

(event EventTick
  (params (DeltaSeconds :type Float%20%28single-precision%29)))

(event Game|Damage|EventAnyDamage
  (params (Damage :type Float%20%28single-precision%29) (DamageType :type Damage%20Type%20Object%20Reference) (InstigatedBy :type Controller%20Object%20Reference) (DamageCauser :type Actor%20Object%20Reference))
  (Development|PrintString (Utilities|String|ToString(Float) (Variables|/Script/GamesGroupProject.PlayerHealthComponent|GetHealth (Variables|Default|GetPlayerHealth)))))

(event Input|AxisEvents|InputAxisLookUp
  (params (AxisValue :type Float%20%28single-precision%29))
  ;[1 1 1] Allows the player to look up and down (on pawn with floating movement componant it makes it fly .....)
)

(event Input|AxisEvents|InputAxisTurn
  (params (AxisValue :type Float%20%28single-precision%29))
  ;[1 1 1] Turning left and right
  (Pawn|Input|AddControllerYawInput AxisValue))

(fn ConstructionScript)